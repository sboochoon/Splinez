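; BP_RFoliageVolume is a foliage volume actor that randomizes its fixed set of tree and grass components on BeginPlay.
; Each of four trees gets a random mesh from the Meshes array and a random X/Y position within the Volume box extent.
; Nine grass components get random yaw and non-uniform scale, plus dynamic materials that vary the "world position color" parameter as a random scalar and a fixed-hue, random-saturation color.
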(event EventBeginPlay
  (bind _returnvalue (Math|Random|RandomFloatinRange 8.0 17.0))
  (bind _meshes (Variables|Default|GetMeshes))
  (bind _volume (Variables|Default|GetVolume))
  (bind _boxextent (Variables|/Script/Engine.BoxComponent|GetBoxExtent _volume))
  (|CallParentFunction)
  (Utilities|FlowControl|Sequence
    (:then_0
      (for _array_element (Utilities|Array|MakeArray (Variables|Default|GetTree) (Variables|Default|GetTree2) (Variables|Default|GetTree3) (Variables|Default|GetTree4))
        (Components|StaticMesh|SetStaticMesh _array_element (Utilities|Array|Get(acopy) _meshes (Math|Random|RandomIntegerinRange 0 (- (Utilities|Array|Length _meshes) 1))))
        (Transformation|SetRelativeLocation _array_element (Math|Vector|MakeVector (Math|Random|RandomFloatinRange (* (.x _boxextent) -1.0) (.x _boxextent)) (Math|Random|RandomFloatinRange (* (.y _boxextent) -1.0) (.y _boxextent)) 0.0) false true)))
    (:then_1
      (for _array_element_2 (Utilities|Array|MakeArray (Variables|Default|GetGrass) (Variables|Default|GetGrass2) (Variables|Default|GetGrass3) (Variables|Default|GetGrass4) (Variables|Default|GetGrass5) (Variables|Default|GetGrass6) (Variables|Default|GetGrass7) (Variables|Default|GetGrass8) (Variables|Default|GetGrass9))
        (Transformation|SetRelativeRotation _array_element_2 (Math|Rotator|MakeRotator 0.0 0.0 (Math|Random|RandomFloatinRange 0.0 3.6e+02)) false false)
        (Transformation|SetRelativeScale3D _array_element_2 (Math|Vector|MakeVector _returnvalue _returnvalue _returnvalue))
        (bind _returnvalue_2 (Rendering|Material|CreateDynamicMaterialInstance _array_element_2 0 (Rendering|Material|GetMaterial _array_element_2 0) :!class /Script/Engine.PrimitiveComponent))
        (Rendering|Material|SetScalarParameterValue _returnvalue_2 "world position color" (Math|Random|RandomFloatinRange -1.0 1.0) :!class /Script/Engine.MaterialInstanceDynamic)
        (Rendering|Material|SetVectorParameterValue _returnvalue_2 "world position color" (Class|KismetMathLibrary|HSVtoRGB 40.6 (Math|Random|RandomFloat) 1.0 1.0) :!class /Script/Engine.MaterialInstanceDynamic)))))

(fn ConstructionScript
  (|CallParentFunction))