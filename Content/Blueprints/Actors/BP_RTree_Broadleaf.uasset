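; BP_RTree_Broadleaf is a broadleaf tree actor that picks its appearance at random when play begins.
; After running the parent's BeginPlay, it sets its static mesh to an entry drawn from the Meshes array using the RandomObjectStream random stream.
; The construction script only calls the parent, so the mesh choice happens at runtime.
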(event EventBeginPlay
  (bind _meshes (Variables|Default|GetMeshes))
  (|CallParentFunction)
  (Components|StaticMesh|SetStaticMesh (Variables|Default|GetStaticMesh) (Utilities|Array|Get(acopy) _meshes (Math|Random|RandomIntegerinRangefromStream 0 (- (Utilities|Array|Length _meshes) 1) (Variables|Default|GetRandomObjectStream)))))

(event Collision|EventActorBeginOverlap
  (params (OtherActor :type Actor%20Object%20Reference))
  (|CallParentFunction OtherActor) ; This node is disabled and will not be called.\nDrag off pins to build functionality.
)

(event EventTick
  (params (DeltaSeconds :type Float%20%28single-precision%29))
  (|CallParentFunction DeltaSeconds) ; This node is disabled and will not be called.\nDrag off pins to build functionality.
)

(fn ConstructionScript
  (|CallParentFunction))