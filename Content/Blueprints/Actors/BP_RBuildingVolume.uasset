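; Building volume actor that picks a random mesh from its Meshes array at BeginPlay and fits spacing boxes around it.
; Front, left and right spacing boxes are resized and repositioned from the mesh's bounding-box maximum, with side depth also including the front spacing.
; The outer Volume box then derives its width, depth and Y offset from the building and spacing boxes, so the footprint adapts to the chosen mesh.
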(event EventBeginPlay
  (bind _building (Variables|Default|GetBuilding))
  (bind _spacingfront (Variables|Default|GetSpacingFront))
  (bind _meshes (Variables|Default|GetMeshes))
  (bind _volume (Variables|Default|GetVolume))
  (bind _spacingleft (Variables|Default|GetSpacingLeft))
  (bind _spacingright (Variables|Default|GetSpacingRight))
  (bind _spacingfront_2 (Variables|Default|GetSpacingFront))
  (bind _staticmesh (Variables|/Script/Engine.StaticMeshComponent|GetStaticMesh _building))
  (bind _boxextent (Variables|/Script/Engine.BoxComponent|GetBoxExtent _spacingleft))
  (bind _boxextent_2 (Variables|/Script/Engine.BoxComponent|GetBoxExtent _spacingright))
  (bind _boxextent_3 (Variables|/Script/Engine.BoxComponent|GetBoxExtent _spacingfront_2))
  (bind _returnvalue (StaticMesh|GetBoundingBox _staticmesh))
  (bind _returnvalue_2 (+ (.y _boxextent_3) (.y (.max _returnvalue))))
  (|CallParentFunction)
  (Components|StaticMesh|SetStaticMesh _building (Utilities|Array|Get(acopy) _meshes (Math|Random|RandomIntegerinRange 0 (- (Utilities|Array|Length _meshes) 1))))
  (Components|Box|SetBoxExtent _spacingfront_2 (Math|Vector|MakeVector (.x (.max _returnvalue)) (.y _boxextent_3) (.z _boxextent_3)) true)
  (Transformation|SetRelativeLocation _spacingfront_2 (Math|Vector|MakeVector 0.0 _returnvalue_2 0.0) false true)
  (Components|Box|SetBoxExtent _spacingleft (Math|Vector|MakeVector (.x _boxextent) _returnvalue_2 (.z _boxextent)) true)
  (Transformation|SetRelativeLocation _spacingleft (Math|Vector|MakeVector (* (+ (.x _boxextent) (.x (.max _returnvalue))) -1.0) 0.0 0.0) false true)
  (Components|Box|SetBoxExtent _spacingright (Math|Vector|MakeVector (.x _boxextent_2) _returnvalue_2 (.z _boxextent_2)) true)
  (Transformation|SetRelativeLocation _spacingright (Math|Vector|MakeVector (+ (.x _boxextent_2) (.x (.max _returnvalue))) 0.0 0.0) false true)
  (Components|Box|SetBoxExtent _volume (Math|Vector|MakeVector (+ (.x (Variables|/Script/Engine.BoxComponent|GetBoxExtent (Variables|Default|GetSpacingLeft))) (.x (.max _returnvalue)) (.x (Variables|/Script/Engine.BoxComponent|GetBoxExtent (Variables|Default|GetSpacingRight)))) (+ (.y (.max _returnvalue)) (.y (Variables|/Script/Engine.BoxComponent|GetBoxExtent _spacingfront))) (.z (Variables|/Script/Engine.BoxComponent|GetBoxExtent _volume))) true)
  (Transformation|SetRelativeLocation _volume (Math|Vector|MakeVector 0.0 (/ (+ (.y (Variables|/Script/Engine.SceneComponent|GetRelativeLocation _spacingfront)) (.y (Variables|/Script/Engine.SceneComponent|GetRelativeLocation (Variables|Default|GetBuilding)))) 4.0) 0.0) false true))

(event Collision|EventActorBeginOverlap
  (params (OtherActor :type Actor%20Object%20Reference))
  (|CallParentFunction OtherActor) ; This node is disabled and will not be called.\nDrag off pins to build functionality.
)

(event EventTick
  (params (DeltaSeconds :type Float%20%28single-precision%29))
  (|CallParentFunction DeltaSeconds) ; This node is disabled and will not be called.\nDrag off pins to build functionality.
)

(fn ConstructionScript
  (|CallParentFunction))