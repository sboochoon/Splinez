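; BP_RHouseVolume is a randomized house actor that sizes box volumes around its building for front and side spacing.
; On BeginPlay it picks the Building mesh from Meshes using RandomObjectStream, a seedable random stream.
; It then resizes and repositions the front, left and right spacing boxes from the mesh bounds.
; The overall Volume box is derived from those bounds and spacing extents, offset along Y toward the front.
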(event EventBeginPlay
  (bind _spacingfront (Variables|Default|GetSpacingFront))
  (bind _meshes (Variables|Default|GetMeshes))
  (bind _building (Variables|Default|GetBuilding))
  (bind _volume (Variables|Default|GetVolume))
  (bind _spacingleft (Variables|Default|GetSpacingLeft))
  (bind _spacingright (Variables|Default|GetSpacingRight))
  (bind _spacingfront_2 (Variables|Default|GetSpacingFront))
  (bind _staticmesh (Variables|/Script/Engine.StaticMeshComponent|GetStaticMesh _building))
  (bind _boxextent (Variables|/Script/Engine.BoxComponent|GetBoxExtent _spacingfront))
  (bind _boxextent_2 (Variables|/Script/Engine.BoxComponent|GetBoxExtent _spacingleft))
  (bind _boxextent_3 (Variables|/Script/Engine.BoxComponent|GetBoxExtent _spacingright))
  (bind _boxextent_4 (Variables|/Script/Engine.BoxComponent|GetBoxExtent _spacingfront_2))
  (bind _returnvalue (StaticMesh|GetBounds _staticmesh))
  (bind _returnvalue_2 (+ (.y _boxextent_4) (.y (.boxextent _returnvalue))))
  (bind _returnvalue_3 (+ (.y (.boxextent _returnvalue)) (.y _boxextent)))
  (|CallParentFunction)
  (Components|StaticMesh|SetStaticMesh _building (Utilities|Array|Get(acopy) _meshes (Math|Random|RandomIntegerinRangefromStream 0 (- (Utilities|Array|Length _meshes) 1) (Variables|Default|GetRandomObjectStream))))
  (Components|Box|SetBoxExtent _spacingfront_2 (Math|Vector|MakeVector (.x (.boxextent _returnvalue)) (.y _boxextent_4) (.z _boxextent_4)) true)
  (Transformation|SetRelativeLocation _spacingfront_2 (Math|Vector|MakeVector 0.0 _returnvalue_2 0.0) false true)
  (Components|Box|SetBoxExtent _spacingleft (Math|Vector|MakeVector (.x _boxextent_2) _returnvalue_2 (.z _boxextent_2)) true)
  (Transformation|SetRelativeLocation _spacingleft (Math|Vector|MakeVector (* (+ (.x _boxextent_2) (.x (.boxextent _returnvalue))) -1.0) 0.0 0.0) false true)
  (Components|Box|SetBoxExtent _spacingright (Math|Vector|MakeVector (.x _boxextent_3) _returnvalue_2 (.z _boxextent_3)) true)
  (Transformation|SetRelativeLocation _spacingright (Math|Vector|MakeVector (+ (.x _boxextent_3) (.x (.boxextent _returnvalue))) 0.0 0.0) false true)
  (Components|Box|SetBoxExtent _volume (Math|Vector|MakeVector (+ (.x (Variables|/Script/Engine.BoxComponent|GetBoxExtent (Variables|Default|GetSpacingLeft))) (.x (.boxextent _returnvalue)) (.x (Variables|/Script/Engine.BoxComponent|GetBoxExtent (Variables|Default|GetSpacingRight)))) _returnvalue_3 (.z (Variables|/Script/Engine.BoxComponent|GetBoxExtent _volume))) true)
  (Transformation|SetRelativeLocation _volume (Math|Vector|MakeVector 0.0 (/ _returnvalue_3 2.0) 0.0) false true))

(event Collision|EventActorBeginOverlap
  (params (OtherActor :type Actor%20Object%20Reference))
  (|CallParentFunction OtherActor) ; This node is disabled and will not be called.\nDrag off pins to build functionality.
)

(event EventTick
  (params (DeltaSeconds :type Float%20%28single-precision%29))
  (|CallParentFunction DeltaSeconds) ; This node is disabled and will not be called.\nDrag off pins to build functionality.
)

(fn ConstructionScript
  (|CallParentFunction))