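; BP_UVRescale creates dynamic material instances for the static mesh actor that owns it, though no UV rescaling logic is present yet.
; On BeginPlay it clears DynamicMaterial and stops unless the owner is a StaticMeshActor.
; It loops over the component's material slots, creating instances from the mesh asset's materials and storing them in the array.
; No parameters are set, and Tick is empty.
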(event EventBeginPlay
  (Utilities|Array|Clear (Variables|Default|GetDynamicMaterial))
  (bind _asstatic_mesh_actor (Utilities|Casting|CastToStaticMeshActor (Components|GetOwner)))
  (bind _output_get (Variables|Default|SetMesh (Variables|/Script/Engine.StaticMeshComponent|GetStaticMesh (Variables|/Script/Engine.StaticMeshActor|GetStaticMeshComponent _asstatic_mesh_actor))))
  (for _index (range 0 (- (Utilities|Array|Length (Rendering|Material|GetMaterials (Variables|/Script/Engine.StaticMeshActor|GetStaticMeshComponent _asstatic_mesh_actor))) 1))
    (bind _returnvalue (Rendering|Material|CreateDynamicMaterialInstance (Rendering|Material|GetMaterial _output_get _index) :!class /Script/Engine.KismetMaterialLibrary))
    (Utilities|Array|Add (Variables|Default|GetDynamicMaterial) _returnvalue)))

(event EventTick
  (params (DeltaSeconds :type Float%20%28single-precision%29)))