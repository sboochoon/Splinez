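; Procedural road generator that builds a randomly winding Lane spline at BeginPlay and lays parallel mesh strips along both sides.
; BuildMainSpline adds points in turning runs that alternate direction, gated by WindingAmount.
; BuildSplineWithMesh chains each new spline off the previous one, offsetting by mesh bounds and random width, then tiles spline meshes from RoadMeshes along it.
; BuildSpline adds extra offset splines for narrower meshes; AddObjectsToSpline is an empty stub.
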(event EventBeginPlay
  (CallFunction|BuildMainSpline)
  (bind _meshwidth (CallFunction|AddMeshtoSpline (Variables|Default|GetLane) "NewEnumerator2" (Math|Random|RandomFloatinRange 2.0 6.0)))
  (Utilities|FlowControl|Sequence
    (:then_0
      (bind (_newspline _meshwidth_2) (CallFunction|BuildSplinewithMesh (Variables|Default|GetLane) _meshwidth "NewEnumerator3" (Math|Random|RandomFloatinRange 1.0 1.5) 0.0 0.0 0.0 false))
      (bind (_newspline_2 _meshwidth_3) (CallFunction|BuildSplinewithMesh _newspline _meshwidth_2 "NewEnumerator0" (Math|Random|RandomFloatinRange 1.0 1.5) 0.0 0.0 0.0 false))
      (bind _newspline_3 (CallFunction|BuildSpline _newspline_2 _meshwidth_3 0.0 0.0 1 false))
      (CallFunction|AddMeshtoSpline _newspline_3 "NewEnumerator1" (Math|Random|RandomFloatinRange 0.25 1.0))
      (bind (_newspline_4 _meshwidth_4) (CallFunction|BuildSplinewithMesh _newspline_2 _meshwidth_3 "NewEnumerator0" (Math|Random|RandomFloatinRange 1.0 1.5) 0.0 0.0 0.0 false))
      (bind (_newspline_5 _meshwidth_5) (CallFunction|BuildSplinewithMesh _newspline_4 _meshwidth_4 "NewEnumerator4" (Math|Random|RandomFloatinRange 1.0 1.5) 0.0 0.0 0.0 false))
      (CallFunction|BuildSplinewithMesh _newspline_5 _meshwidth_5 "NewEnumerator2" (Math|Random|RandomFloatinRange 2.0 4.0) 0.0 0.0 0.0 false))
    (:then_1
      (bind (_newspline_6 _meshwidth_6) (CallFunction|BuildSplinewithMesh (Variables|Default|GetLane) _meshwidth "NewEnumerator4" (Math|Random|RandomFloatinRange 1.0 1.5) 0.0 0.0 0.0 true))
      (bind (_newspline_7 _meshwidth_7) (CallFunction|BuildSplinewithMesh _newspline_6 _meshwidth_6 "NewEnumerator0" (Math|Random|RandomFloatinRange 1.0 1.5) 0.0 0.0 0.0 true))
      (bind _newspline_8 (CallFunction|BuildSpline _newspline_7 _meshwidth_7 0.0 0.0 1 true))
      (CallFunction|AddMeshtoSpline _newspline_8 "NewEnumerator1" (Math|Random|RandomFloatinRange 0.25 1.0))
      (bind (_newspline_9 _meshwidth_8) (CallFunction|BuildSplinewithMesh _newspline_7 _meshwidth_7 "NewEnumerator0" (Math|Random|RandomFloatinRange 1.0 1.5) 0.0 0.0 0.0 true))
      (bind (_newspline_10 _meshwidth_9) (CallFunction|BuildSplinewithMesh _newspline_9 _meshwidth_8 "NewEnumerator3" (Math|Random|RandomFloatinRange 1.0 1.5) 0.0 0.0 0.0 true))
      (CallFunction|BuildSplinewithMesh _newspline_10 _meshwidth_9 "NewEnumerator2" (Math|Random|RandomFloatinRange 2.0 4.0) 0.0 0.0 0.0 true))))

(fn ConstructionScript)

(fn BuildMainSpline
  (if (Math|Random|RandomBool)
    (LocalVariables|SetWindingDirection 1)
    (else
      (LocalVariables|SetWindingDirection -1)))
  (LocalVariables|SetRotationAchieved true)
  ;[0 0.1645 1] Build spline based on num of Points
  (for _index (range 1 (Variables|Default|GetPoints))
    (if (LocalVariables|GetRotationAchieved)
      (LocalVariables|SetCurrentRotation 0.0)
      ;[1 0.9282 0] Higher WindingAmount will apply more rotation on the spline points
      (if (<= (Math|Random|RandomFloat) (Variables|Default|GetWindingAmount))
        (LocalVariables|SetRotationAchieved false)
        (LocalVariables|SetWindingDirection (* (LocalVariables|GetWindingDirection) -1))
        (LocalVariables|SetCurrentRotation (+ (LocalVariables|GetCurrentRotation) (LocalVariables|GetRotationToAdd)))
        (if (>= (LocalVariables|GetCurrentRotation) (Variables|Default|GetMaxRotationAmount))
          (LocalVariables|SetRotationAchieved true)
          (else
            (LocalVariables|SetRotationAchieved false)))
        ;[0.1121 1 0] Function Call
        (CallFunction|RotateandAddPoint _index (* (LocalVariables|GetWindingDirection) (LocalVariables|GetRotationToAdd)) (Variables|Default|GetLane))
        (else
          ;[0.1062 1 0] Function Call
          (CallFunction|RotateandAddPoint _index 0.0 (Variables|Default|GetLane))))
      (else
        (LocalVariables|SetCurrentRotation (+ (LocalVariables|GetCurrentRotation) (LocalVariables|GetRotationToAdd)))
        (if (>= (LocalVariables|GetCurrentRotation) (Variables|Default|GetMaxRotationAmount))
          (LocalVariables|SetRotationAchieved true)
          (else
            (LocalVariables|SetRotationAchieved false)))
        ;[0.1121 1 0] Function Call
        (CallFunction|RotateandAddPoint _index (* (LocalVariables|GetWindingDirection) (LocalVariables|GetRotationToAdd)) (Variables|Default|GetLane))))))

(fn RotateandAddPoint
  (params (Point :type Integer) (RotationAmount :type Float%20%28single-precision%29) (Spline :type Spline%20Component%20Object%20Reference))
  (bind _returnvalue (Spline|GetTangentatSplinePoint Spline Point "Local"))
  (bind _returnvalue_2 (Spline|GetLocationatSplinePoint Spline Point "Local"))
  (bind _returnvalue_3 (Spline|GetRotationatSplinePoint Spline Point "Local"))
  (bind _returnvalue_4 (Class|SplineComponent|GetDirectionatSplinePoint Spline Point "Local"))
  (bind _distancebetweenpoints (Variables|Default|GetDistanceBetweenPoints))
  (bind _maxrotationamount (Variables|Default|GetMaxRotationAmount))
  (bind _returnvalue_5 (Math|Rotator|MakeRotator (.roll _returnvalue_3) (.pitch _returnvalue_3) RotationAmount))
  (bind _returnvalue_6 (Math|Vector|RotateVectorAroundAxis _returnvalue_4 RotationAmount "0, 0,1.000000"))
  (bind _returnvalue_7 (+ (.yaw _returnvalue_3) RotationAmount))
  (bind _returnvalue_8 (* _maxrotationamount -1.0))
  (bind _returnvalue_9 (Math|Vector|RotateVector _returnvalue _returnvalue_5))
  (bind _returnvalue_10 (Math|Rotator|MakeRotator (.roll _returnvalue_3) (.pitch _returnvalue_3) _returnvalue_7))
  (bind _returnvalue_11 (* _returnvalue_6 _distancebetweenpoints))
  (bind _returnvalue_12 (Math|Vector|ClampVectorSize _returnvalue_9 _returnvalue_8 _maxrotationamount))
  (bind _returnvalue_13 (+ _returnvalue_2 _returnvalue_11))
  ;[1 1 1] Debug
  (Development|PrintString (Utilities|String|ToString(Rotator) _returnvalue_10) false false "(R=0.000000,G=0.660000,B=1.000000,A=1.000000)" 9e+01)
  (Development|PrintString (Utilities|String|ToString(Vector) _returnvalue_13) false false "(R=0.034151,G=1.000000,B=0.000000,A=1.000000)" 9e+01)
  (Development|PrintString (Utilities|String|ToString(Vector) _returnvalue_12) false false "(R=1.000000,G=0.000000,B=0.219121,A=1.000000)" 9e+01)
  (Class|SplineComponent|AddPoint Spline (Utilities|Struct|MakeSplinePoint (Math|Conversions|ToFloat(Integer) (+ Point 1)) _returnvalue_13 _returnvalue _returnvalue_12 _returnvalue_10 "1.000000,1.000000,1.000000") true))

(fn BuildSpline
  (params (ReferencedSpline :type Spline%20Component%20Object%20Reference) (RightOffset :type Float%20%28single-precision%29) (ForwardOffset :type Float%20%28single-precision%29) (UpOffset :type Float%20%28single-precision%29) (DecreaseSplineResolutionAmount :type Integer) (PlaceLeft :type Boolean))
  (bind _maxrotationamount (Variables|Default|GetMaxRotationAmount))
  (if PlaceLeft
    (LocalVariables|SetRightVectorOffset (* RightOffset -1.0))
    (else
      (LocalVariables|SetRightVectorOffset RightOffset)))
  (LocalVariables|SetForwardVectorOffset ForwardOffset)
  (LocalVariables|SetUpVectorOffset UpOffset)
  ;[0.375 0.375 0.375] BUILD SPLINE
  ;;[1 1 1] Add a new spline component and clear it's points
  (bind _returnvalue (AddComponent|AddSplineComponent true))
  (bind _output_get (LocalVariables|SetCreatedSpline _returnvalue))
  (Spline|ClearSplinePoints _output_get true)
  (LocalVariables|SetInputKey 0)
  ;;[0 0.1127 1] Loop through number of points from original spline
  (for _index (range 0 (- (Spline|GetNumberOfSplinePoints ReferencedSpline) 1))
    (if (== (Math|Integer|%(Integer) _index DecreaseSplineResolutionAmount) 0)
      ;;[1 1 1] Create new spline point with position, type and tangent
      (Class|SplineComponent|AddPoint (LocalVariables|GetCreatedSpline) (Utilities|Struct|MakeSplinePoint (Math|Conversions|ToFloat(Integer) (LocalVariables|GetInputKey)) (+ (.Location (Spline|GetLocationandTangentatSplinePoint ReferencedSpline _index "World")) (+ (* (Class|SplineComponent|GetRightVectoratSplinePoint ReferencedSpline _index "World") (LocalVariables|GetRightVectorOffset)) (* (Class|SplineComponent|GetUpVectoratSplinePoint ReferencedSpline _index "World") (LocalVariables|GetUpVectorOffset)) (* (Math|Vector|GetForwardVector ReferencedSpline) (LocalVariables|GetForwardVectorOffset)))) (Math|Vector|ClampVectorSize (.Tangent (Spline|GetLocationandTangentatSplinePoint ReferencedSpline _index "World")) (* _maxrotationamount -1.0) _maxrotationamount) (Math|Vector|ClampVectorSize (.Tangent (Spline|GetLocationandTangentatSplinePoint ReferencedSpline _index "World")) (* _maxrotationamount -1.0) _maxrotationamount) (Spline|GetRotationatSplinePoint ReferencedSpline _index "World") "1.000000,1.000000,1.000000" (Class|SplineComponent|GetSplinePointType ReferencedSpline _index)) true)
      (Math|Integer|IncrementInt (LocalVariables|GetInputKey))))
  ;[1 0 0] Return the new spline
  (return (LocalVariables|GetCreatedSpline)))

(fn AddMeshtoSpline
  (params (Spline :type Spline%20Component%20Object%20Reference) (Mesh :type BP_MeshNames%20Enum :default "NewEnumerator0") (Width :type Float%20%28single-precision%29))
  (bind _distancebetweenpoints (Variables|Default|GetDistanceBetweenPoints))
  (bind _tangentscale (LocalVariables|GetTangentScale))
  (Utilities|FlowControl|Sequence
    (:then_0
      ;[1 1 1] Set the mesh based on what we entered in "Mesh"
      (for _array_element (Variables|Default|GetRoadMeshes)
        (if (Utilities|Name|Equal(Name) (.title _array_element) (Utilities|String|StringToName (Utilities|String|EnumtoString Mesh)))
          (LocalVariables|SetMeshToUse (.mesh _array_element))))
      ;[0 0.1195 1] Loop through spline points to points-2 (because we're grabbing the next point to set the end position and tangent)
      (for _index (range 0 (- (Spline|GetNumberOfSplinePoints Spline) 2))
        ;[1 1 1] Create a mesh component and set the tag and mesh
        (bind _returnvalue (AddComponent|AddSplineMeshComponent false))
        (Components|StaticMesh|SetStaticMesh _returnvalue (LocalVariables|GetMeshToUse))
        ;[1 1 1] Set scale for the mesh to be the width
        (SplineMesh|SetStartScale _returnvalue (Math|Vector2D|MakeVector2D Width 1.0) true :!class /Script/Engine.SplineMeshComponent)
        (SplineMesh|SetEndScale _returnvalue (Math|Vector2D|MakeVector2D Width 1.0) true :!class /Script/Engine.SplineMeshComponent)
        ;[1 1 1] Set the position and tangent info for the mesh
        (SplineMesh|SetStartandEnd _returnvalue (Spline|GetLocationatDistanceAlongSpline Spline (* _index _distancebetweenpoints) "World") (* (Spline|GetDirectionatDistanceAlongSpline Spline (* _index _distancebetweenpoints) "World") _tangentscale) (Spline|GetLocationatDistanceAlongSpline Spline (* (+ _index 1) _distancebetweenpoints) "World") (* (Spline|GetDirectionatDistanceAlongSpline Spline (* (+ _index 1) _distancebetweenpoints) "World") _tangentscale) true :!class /Script/Engine.SplineMeshComponent)))
    (:then_1
      ;[1 0 0] Return the mesh width of current spline based on the mesh and the width value we gave it
      (Development|PrintString (Utilities|String|ToString(Float) (* (.y (.boxextent (StaticMesh|GetBounds (LocalVariables|GetMeshToUse)))) Width)) false false "(R=0.916948,G=0.000000,B=1.000000,A=1.000000)" 2e+01)
      (return (* (.y (.boxextent (StaticMesh|GetBounds (LocalVariables|GetMeshToUse)))) Width)))))

(fn BuildSplinewithMesh
  (params (ReferencedSpline :type Spline%20Component%20Object%20Reference) (ReferencedSplineMeshWidth :type Float%20%28single-precision%29) (Mesh :type BP_MeshNames%20Enum :default "NewEnumerator0") (Width :type Float%20%28single-precision%29) (RightOffset :type Float%20%28single-precision%29) (ForwardOffset :type Float%20%28single-precision%29) (UpOffset :type Float%20%28single-precision%29) (PlaceLeft :type Boolean))
  (bind _distancebetweenpoints (Variables|Default|GetDistanceBetweenPoints))
  (bind _tangentscale (LocalVariables|GetTangentScale))
  (bind _maxrotationamount (Variables|Default|GetMaxRotationAmount))
  (Utilities|FlowControl|Sequence
    (:then_0
      ;[0.2969 0.2969 0.2969] SET VALUES
      ;;[1 1 1] Find the appropriate mesh
      (for _array_element (Variables|Default|GetRoadMeshes)
        (if (Utilities|Name|Equal(Name) (.title _array_element) (Utilities|String|StringToName (Utilities|String|EnumtoString Mesh)))
          (LocalVariables|SetMeshToUse (.mesh _array_element))))
      ;;[1 1 1] Set offset either left or right of the currently referenced spline based on user input
      (if PlaceLeft
        (LocalVariables|SetRightVectorOffset (* (+ (+ ReferencedSplineMeshWidth (/ (* (* (.y (.boxextent (StaticMesh|GetBounds (LocalVariables|GetMeshToUse)))) 2.0) Width) 2.0)) RightOffset) -1.0))
        (else
          (Development|PrintString (Utilities|String|ToString(Float) (+ (+ ReferencedSplineMeshWidth (/ (* (* (.y (.boxextent (StaticMesh|GetBounds (LocalVariables|GetMeshToUse)))) 2.0) Width) 2.0)) RightOffset)) false false "(R=0.000000,G=1.000000,B=0.194615,A=1.000000)" 15.0)
          (LocalVariables|SetRightVectorOffset (+ (+ ReferencedSplineMeshWidth (/ (* (* (.y (.boxextent (StaticMesh|GetBounds (LocalVariables|GetMeshToUse)))) 2.0) Width) 2.0)) RightOffset)))))
    (:then_1
      ;[0.375 0.375 0.375] BUILD SPLINE
      ;;[1 1 1] Add a new spline component and clear it's points
      (bind _returnvalue (AddComponent|AddSplineComponent true))
      (bind _output_get (LocalVariables|SetCreatedSpline _returnvalue))
      (Spline|ClearSplinePoints _returnvalue true)
      ;;[0 0.1127 1] Loop through number of points from original spline
      (for _index (range 0 (- (Spline|GetNumberOfSplinePoints ReferencedSpline) 1))
        ;;[1 1 1] Create new spline point with position, type and tangent
        (Class|SplineComponent|AddPoint (LocalVariables|GetCreatedSpline) (Utilities|Struct|MakeSplinePoint (Math|Conversions|ToFloat(Integer) _index) (+ (.Location (Spline|GetLocationandTangentatSplinePoint ReferencedSpline _index "World")) (+ (* (Class|SplineComponent|GetRightVectoratSplinePoint ReferencedSpline _index "World") (LocalVariables|GetRightVectorOffset)) (* (Class|SplineComponent|GetUpVectoratSplinePoint ReferencedSpline _index "World") UpOffset) (* (Math|Vector|GetForwardVector ReferencedSpline) ForwardOffset))) (Math|Vector|ClampVectorSize (.Tangent (Spline|GetLocationandTangentatSplinePoint ReferencedSpline _index "World")) (* _maxrotationamount -1.0) _maxrotationamount) (Math|Vector|ClampVectorSize (.Tangent (Spline|GetLocationandTangentatSplinePoint ReferencedSpline _index "World")) (* _maxrotationamount -1.0) _maxrotationamount) (Spline|GetRotationatSplinePoint ReferencedSpline _index "World") "1.000000,1.000000,1.000000" (Class|SplineComponent|GetSplinePointType ReferencedSpline _index)) true)))
    (:then_2
      ;[0.3646 0.3646 0.3646] ADD MESH TO SPLINE
      ;;[0 0.1195 1] Loop through spline points to points-2 (because we're grabbing the next point to set the end position and tangent)
      (for _index_2 (range 0 (- (Spline|GetNumberOfSplinePoints (LocalVariables|GetCreatedSpline)) 2))
        ;;[1 1 1] Create a mesh component and set the tag and mesh
        (bind _returnvalue_2 (AddComponent|AddSplineMeshComponent false))
        (Components|StaticMesh|SetStaticMesh _returnvalue_2 (LocalVariables|GetMeshToUse))
        ;;[1 1 1] Set scale for the mesh to be the width
        (SplineMesh|SetStartScale _returnvalue_2 (Math|Vector2D|MakeVector2D Width 1.0) true :!class /Script/Engine.SplineMeshComponent)
        (SplineMesh|SetEndScale _returnvalue_2 (Math|Vector2D|MakeVector2D Width 1.0) true :!class /Script/Engine.SplineMeshComponent)
        ;;[1 1 1] Set the position and tangent info for the mesh
        (SplineMesh|SetStartandEnd _returnvalue_2 (Spline|GetLocationatDistanceAlongSpline (LocalVariables|GetCreatedSpline) (* _index_2 _distancebetweenpoints) "World") (* (Spline|GetDirectionatDistanceAlongSpline (LocalVariables|GetCreatedSpline) (* _index_2 _distancebetweenpoints) "World") _tangentscale) (Spline|GetLocationatDistanceAlongSpline (LocalVariables|GetCreatedSpline) (* (+ _index_2 1) _distancebetweenpoints) "World") (* (Spline|GetDirectionatDistanceAlongSpline (LocalVariables|GetCreatedSpline) (* (+ _index_2 1) _distancebetweenpoints) "World") _tangentscale) true :!class /Script/Engine.SplineMeshComponent)))
    (:then_3
      ;[0.3698 0.3698 0.3698] RETURN VALUES
      ;;[1 1 1] Get the mesh size based on Y bounds and width
      (Development|PrintString (Utilities|String|ToString(Float) (* Width (.y (.boxextent (StaticMesh|GetBounds (LocalVariables|GetMeshToUse)))))) false false "(R=1.000000,G=0.000000,B=0.188499,A=1.000000)" 15.0)
      ;;[1 0 0] Return the new spline
      (return (LocalVariables|GetCreatedSpline) (* Width (.y (.boxextent (StaticMesh|GetBounds (LocalVariables|GetMeshToUse)))))))))

(fn AddObjectstoSpline
  (params (ReferencedSpline :type Spline%20Component%20Object%20Reference)))